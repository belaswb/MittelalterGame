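; Base AI NPC character for the MMO, handling threat-based targeting, death rewards and respawning.
; Server damage events accumulate aggro in parallel character and value arrays, attack the highest entry and register the NPC in players' combat lists.
; Death clears those combat links, grants loot rights and quest kill progress to the top-aggro player, and starts a respawn timer.
; Respawn restores spawn transform and health, empties inventory and aggro, and multicasts a hostility reset.
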(event Custom|RespawnMulticast
  ;[1 1 1] Multicast: Respawn
  (Variables|Default|SetHostility "NewEnumerator1"))

(event Custom|Respawn%20Server
  ;[1 1 1] Server side: Respawn
  (Utilities|Array|Clear (Variables|Default|GetInventory))
  (Transformation|SetActorTransform (Variables|Default|GetSpawnLocation))
  (Variables|Default|SetHP (Variables|Default|GetMaxHP))
  (Rendering|SetActorHiddenInGame false)
  (CallFunction|ClearAggro)
  (CallFunction|RespawnMulticast))

(event EventAssignTarget
  (params (TargetToAssign :type BP%20MMO%20Character%20Object%20Reference))
  ;[1 1 1] both: Assign Target
  (Variables|Default|SetCurrentTarget TargetToAssign))

(event EventOnDeathServer
  ;[0.94 0.4685 0.3196] Server side: on NPC death
  (Utilities|Time|SetTimerbyEvent (delegate Custom|Respawn%20Server) (Variables|Default|GetRespawnTime))
  (CallFunction|StopAttacking)
  ;[1 1 1] Remove self from players' InCombatWith lists
  (for _array_element (Variables|Default|GetAggroCharacters)
    (bind _asbp_mmoplayer_character (Utilities|Casting|CastToBP_MMOPlayerCharacter _array_element))
    (Utilities|Array|RemoveItem (Variables|/Game/MMO/Blueprints/BP_MMOPlayerCharacter.BP_MMOPlayerCharacter_C|GetInCombatWith _asbp_mmoplayer_character) self))
  ;[0.851 0.299 0] Grant loot rights to highest aggro player
  (bind _mmocharacter (CallFunction|HighestAggroCharacter))
  (Utilities|Array|Add (Variables|Default|GetLootRights) _mmocharacter)
  (Default|GrantLootRights _mmocharacter self)
  ;[0.09093 1 0.3993] Update kill quest progress
  (bind _asbp_mmoplayer_character_2 (Utilities|Casting|CastToBP_MMOPlayerCharacter _mmocharacter))
  (for (_array_element_2 _array_index) (Variables|/Game/MMO/Blueprints/BP_MMOPlayerCharacter.BP_MMOPlayerCharacter_C|GetAcceptedQuests _asbp_mmoplayer_character_2) ; for each accepted quest
    (bind (_array_element_3 _array_index_2) (Utilities|Array|ForEachLoopwithBreak (Variables|/Script/MMO.Quest|GetKillTasks (.Quest (Utilities|Struct|BreakFAcceptedQuest _array_element_2))) :!label _label)
      (:LoopBody
        (if (and (== (.CharacterToKill (Utilities|Struct|BreakQuestTaskKill _array_element_3)) (Utilities|GetClass self)) (< (Utilities|Array|Get(acopy) (.TaskProgress (Utilities|Struct|BreakFAcceptedQuest _array_element_2)) _array_index_2) (.NumberOfKills (Utilities|Struct|BreakQuestTaskKill _array_element_3))))
          (bind _output_get (Variables|Default|SetTemp (.TaskProgress (Utilities|Struct|BreakFAcceptedQuest _array_element_2))))
          (Utilities|Array|SetArrayElem _output_get _array_index_2 (+ (Utilities|Array|Get(acopy) (.TaskProgress (Utilities|Struct|BreakFAcceptedQuest _array_element_2)) _array_index_2) 1))
          (Utilities|Array|SetArrayElem (Variables|/Game/MMO/Blueprints/BP_MMOPlayerCharacter.BP_MMOPlayerCharacter_C|GetAcceptedQuests _asbp_mmoplayer_character_2) _array_index (Utilities|Struct|MakeFAcceptedQuest (.Quest (Utilities|Struct|BreakFAcceptedQuest _array_element_2)) (Variables|Default|GetTemp)))
          (Default|UpdateAcceptedCompletedQuests _asbp_mmoplayer_character_2 (Variables|/Game/MMO/Blueprints/BP_MMOPlayerCharacter.BP_MMOPlayerCharacter_C|GetAcceptedQuests _asbp_mmoplayer_character_2) (Variables|/Game/MMO/Blueprints/BP_MMOPlayerCharacter.BP_MMOPlayerCharacter_C|GetCompletedQuests _asbp_mmoplayer_character_2))
          (goto _label Break))))))

(event EventOnDamageReceivedServer
  (params (Damage%20Amount :type Integer) (Damage%20Source :type BP%20MMO%20Character%20Object%20Reference))
  ;[1 1 1] Server side: Add aggro when this NPC is dealt damage
  (if (> (Variables|Default|GetHP) 0) ; if alive
    (CallFunction|AddAggro Damage%20Source Damage%20Amount)
    ;[1 1 1] Add this AI to player's InCombatWith list
    (bind _asbp_mmoplayer_character (Utilities|Casting|CastToBP_MMOPlayerCharacter Damage%20Source))
    (Utilities|Array|Add (Variables|/Game/MMO/Blueprints/BP_MMOPlayerCharacter.BP_MMOPlayerCharacter_C|GetInCombatWith _asbp_mmoplayer_character) self)))

(event EventBeginPlay
  ;[1 1 1] Server side: Remember spawn location
  (|CallParentFunction)
  (Networking|SwitchHasAuthority
    (:Authority
      (Variables|Default|SetSpawnLocation (Transformation|GetActorTransform)))))

(fn ConstructionScript)

(fn AddAggro
  (params (Character :type BP%20MMO%20Character%20Object%20Reference) (Aggro :type Integer))
  (LocalVariables|SetMMOCharacter Character)
  (LocalVariables|SetAggroValue Aggro)
  (bind (_array_element _array_index) (Utilities|Array|ForEachLoopwithBreak (Variables|Default|GetAggroCharacters) :!label _label)
    (:LoopBody
      (if (== _array_element (LocalVariables|GetMMOCharacter))
        (Utilities|FlowControl|Sequence
          (:then_0
            (goto _label Break))
          (:then_1
            (LocalVariables|SetCharacterIndex _array_index)
            ;[1 1 1] Add to existing entry
            (Utilities|Array|SetArrayElem (Variables|Default|GetAggroValues) (LocalVariables|GetCharacterIndex) (+ (Utilities|Array|Get(acopy) (Variables|Default|GetAggroValues) (LocalVariables|GetCharacterIndex)) (LocalVariables|GetAggroValue)))
            (CallFunction|ChooseAttackTarget :!label _label_2)))))
    (:Completed
      ;[1 1 1] Create a new entry
      (Utilities|Array|Add (Variables|Default|GetAggroCharacters) (LocalVariables|GetMMOCharacter))
      (Utilities|Array|Add (Variables|Default|GetAggroValues) (LocalVariables|GetAggroValue))
      (goto _label_2))))

(fn HighestAggroCharacter
  (bind _aggrovalues (Variables|Default|GetAggroValues))
  (bind (_indexofmaxvalue _maxvalue) (Math|Integer|MaxOfIntArray _aggrovalues))
  (return (Utilities|Array|Get(acopy) (Variables|Default|GetAggroCharacters) _indexofmaxvalue) _maxvalue))

(fn ChooseAttackTarget
  (bind (_mmocharacter _highestaggro) (CallFunction|HighestAggroCharacter))
  (if (> _highestaggro 0)
    (CallFunction|Attack _mmocharacter)
    (else
      (CallFunction|StopAttacking))))

(fn ClearAggro
  (Utilities|Array|Clear (Variables|Default|GetAggroCharacters))
  (Utilities|Array|Clear (Variables|Default|GetAggroValues))
  (Variables|Default|SetinCombat false)
  (Variables|Default|SetCurrentTarget 0))