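; BP_AssetReferencer is a Blueprint that holds arrays of quest and hotbar item asset references, with debug helpers to print them.
; PrintAssetPath prints a valid asset's object name, despite its name, or reports it as invalid.
; A disconnected chain would print the combined count and each entry of both arrays, but it never runs.
; BeginPlay and the construction script are empty, and nothing in these graphs calls the helper at runtime.
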(event Custom|PrintAssetPath
  (params (Obj :type Object%20Object%20Reference))
  (if (Utilities|IsValid Obj)
    (Development|PrintString (Utilities|String|Append "Asset: " (Utilities|GetObjectName Obj)))
    (else
      (Development|PrintString "Invalid asset"))))

(event EventBeginPlay)

(fn ConstructionScript)