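; BP_WorldItem is a clickable item placed in the world that the player can pick up.
; Clicking it passes the actor to PickUpItem on player 0's BP_MMOPlayerCharacter.
; Its static mesh comes from the Item data, applied in the Construction Script on the authority and at BeginPlay on remote clients.
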(event MouseInput|EventActorOnClicked
  (params (ButtonPressed :type Key%20Structure :default "None"))
  (Default|PickUpItem (.AsBP%20MMOPlayer%20Character (Utilities|Casting|CastToBP_MMOPlayerCharacter (Game|GetPlayerCharacter 0))) self))

(event EventBeginPlay
  (Networking|SwitchHasAuthority
    (:Remote
      (Components|StaticMesh|SetStaticMesh (Variables|/Script/MMO.ItemData|GetMesh (Variables|Default|GetItem))))))

(event Collision|EventActorBeginOverlap
  (params (OtherActor :type Actor%20Object%20Reference)))

(event EventTick
  (params (DeltaSeconds :type Float%20%28single-precision%29)))

(fn ConstructionScript
  (Networking|SwitchHasAuthority
    (:Authority
      (Components|StaticMesh|SetStaticMesh (Variables|/Script/MMO.ItemData|GetMesh (Variables|Default|GetItem))))))