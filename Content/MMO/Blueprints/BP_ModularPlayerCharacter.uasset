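; Modular MMO player character that wears armor on five body slots and uses items or abilities from a hotbar on keys 1-4.
; Equipping moves items between inventory and slot variables and updates the equipment UI.
; RepNotifies on those slots swap each part's mesh and material, falling back to underwear when empty.
; Head, legs, hands and feet follow the main (chest) mesh via master pose, with dynamic materials created for highlighting.
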(event Custom|Equip
  (params (Inventory%20Slot :type Integer))
  ;[1 0.848 0.3919] Equipping
  (bind (_inventoryitem _hasitem _arrayindex) (CallFunction|FindInventoryStackbySlotIndex Inventory%20Slot))
  (bind _asequipment (Utilities|Casting|CastToEquipment (.Item (Utilities|Struct|BreakFInventoryItem _inventoryitem))))
  (Utilities|FlowControl|Sequence
    (:then_0
      ;[1 0.848 0.3919] If some equipment was already on, place the old item back in the inventory
      (Utilities|IsValid (Utilities|Select :Index (Variables|/Script/MMO.Equipment|GetType _asequipment) :Head (Variables|Default|GetEquippedHead) :Torso (Variables|Default|GetEquippedChest) :Legs (Variables|Default|GetEquippedLegs) :Hands (Variables|Default|GetEquippedHands) :Feet (Variables|Default|GetEquippedFeet) :Weapon 0 :WeaponSecondary 0)
        (:Is%20Valid
          (Utilities|Array|Add (Variables|Default|GetInventory) (Utilities|Struct|MakeFInventoryItem (Utilities|Select :Index (Variables|/Script/MMO.Equipment|GetType _asequipment) :Head (Variables|Default|GetEquippedHead) :Torso (Variables|Default|GetEquippedChest) :Legs (Variables|Default|GetEquippedLegs) :Hands (Variables|Default|GetEquippedHands) :Feet (Variables|Default|GetEquippedFeet) :Weapon 0 :WeaponSecondary 0) 1 Inventory%20Slot)))))
    (:then_1
      (CallFunction|EquipItem _asequipment))
    (:then_2
      (Utilities|Array|RemoveIndex (Variables|Default|GetInventory) _arrayindex)
      (CallFunction|UpdateInventory (Variables|Default|GetInventory)))))

(event Custom|EquipUnderwear
  (params (ArmorType :type EquipmentType%20Enum :default "Head"))
  (bind _head (Variables|Default|GetHead))
  (bind _feet (Variables|Default|GetFeet))
  (bind _hands (Variables|Default|GetHands))
  (bind _legs (Variables|Default|GetLegs))
  (bind _mesh (Variables|Character|GetMesh))
  (bind _returnvalue (Utilities|Select :Index ArmorType :Head _head :Torso _mesh :Legs _legs :Hands _hands :Feet _feet :Weapon 0 :WeaponSecondary 0))
  ;[1 0.848 0.3919] Client: Equip Underwear
  (Class|SkinnedMeshComponent|SetSkeletalMesh _returnvalue (Utilities|Select :Index ArmorType :Head "/Game/MMO/Characters/Mannequin/Modular/SK_Head.SK_Head" :Torso "/Game/MMO/Characters/Mannequin/Modular/SK_Chest.SK_Chest" :Legs "/Game/MMO/Characters/Mannequin/Modular/SK_Legs.SK_Legs" :Hands "/Game/MMO/Characters/Mannequin/Modular/SK_Hands.SK_Hands" :Feet "/Game/MMO/Characters/Mannequin/Modular/SK_Feet.SK_Feet" :Weapon 0 :WeaponSecondary 0) true)
  (Rendering|Material|SetMaterial _returnvalue 0 "/Game/MMO/Characters/Mannequin/Materials/M_UE4Man_Body.M_UE4Man_Body"))

(event Custom|UseItem
  (params (Index :type Integer))
  ;[1 0.6005 0.1372] Use Item
  (bind _inventoryitem (CallFunction|FindInventoryStackbySlotIndex Index))
  (Utilities|Casting|CastToEquipment (.Item (Utilities|Struct|BreakFInventoryItem _inventoryitem)))
  (CallFunction|Equip Index))

(event Custom|PlaceOnHotbar
  (params (Object :type Hotbar%20Object%20Object%20Reference) (Index :type Integer) (OldIndex :type Integer))
  ;[0.996 1 0.3327] Set hotbar ability or item
  (Utilities|Array|SetArrayElem (Variables|Default|GetHotbar) Index Object)
  (Utilities|FlowControl|Sequence
    (:then_0
      ;[0.996 1 0.3327] clear old slot if needed
      (Math|Integer|CompareInt OldIndex -1
        (:>
          (Utilities|Array|SetArrayElem (Variables|Default|GetHotbar) OldIndex 0))))
    (:then_1
      (CallFunction|UpdateHotbar (Variables|Default|GetHotbar)))))

(event Custom|ClearHotbarSlot
  (params (Index :type Integer))
  ;[0.996 1 0.3327] Clear hotbar slot
  (Utilities|Array|SetArrayElem (Variables|Default|GetHotbar) Index 0)
  (CallFunction|UpdateHotbar (Variables|Default|GetHotbar)))

(event Custom|UseHotbarSlot
  (params (Index :type Integer) (CurrentTarget :type BP%20MMO%20Character%20Object%20Reference))
  (bind _hotbar (Variables|Default|GetHotbar))
  (bind _output (Utilities|Array|Get(acopy) _hotbar Index))
  (if (> (Variables|Default|GetHP) 0) ; check that the character is alive
    ;[1 0.6005 0.1372] Use hotbar item
    (bind _asitem_data (Utilities|Casting|CastToItemData _output)
      (:then
        (CallFunction|UseHotbarItem _asitem_data))
      (:CastFailed
        ;[0.996 1 0.3327] Use hotbar ability
        (bind _asability (Utilities|Casting|CastToAbility _output))
        (CallFunction|UseAbility _asability CurrentTarget)))))

(event Custom|ConfirmEquip
  (params (ItemToEquip :type F%20Inventory%20Item%20Structure))
  ;[1 0.848 0.3919] Equipping
  (Default|EquipItem (Variables|/Game/MMO/Blueprints/UserInterface/WBP_FullUI.WBP_FullUI_C|GetEquipment (Variables|/Game/MMO/Blueprints/BP_MMOInstance.BP_MMOInstance_C|GetFullUIWidget (Utilities|MMOInstance))) ItemToEquip))

(event Custom|Unequip
  (params (Equipment :type Equipment%20Object%20Reference))
  (bind _inventory (Variables|Default|GetInventory))
  ;[1 0.848 0.3919] Unequip
  (bind _output (CallFunction|GetEmptyInventorySlot))
  (Utilities|Array|Add _inventory (Utilities|Struct|MakeFInventoryItem Equipment 1 _output))
  (CallFunction|UpdateInventory _inventory)
  (switch Utilities|FlowControl|Switch|SwitchonEquipmentType (Variables|/Script/MMO.Equipment|GetType Equipment)
    (:Head
      (Variables|Default|SetEquippedHead 0))
    (:Torso
      (Variables|Default|SetEquippedChest 0))
    (:Legs
      (Variables|Default|SetEquippedLegs 0))
    (:Hands
      (Variables|Default|SetEquippedHands 0))
    (:Feet
      (Variables|Default|SetEquippedFeet 0))))

(event Custom|EquipArmor
  (params (ArmorToEquip :type Equipment%20Object%20Reference))
  (bind _equippedmesh (Variables|/Script/MMO.Equipment|GetEquippedMesh ArmorToEquip))
  (bind _type (Variables|/Script/MMO.Equipment|GetType ArmorToEquip))
  (bind _materialoverride (Variables|/Script/MMO.Equipment|GetMaterialOverride ArmorToEquip))
  (bind _head (Variables|Default|GetHead))
  (bind _feet (Variables|Default|GetFeet))
  (bind _hands (Variables|Default|GetHands))
  (bind _legs (Variables|Default|GetLegs))
  (bind _mesh (Variables|Character|GetMesh))
  (bind _returnvalue (Utilities|Select :Index _type :Head _head :Torso _mesh :Legs _legs :Hands _hands :Feet _feet :Weapon 0 :WeaponSecondary 0))
  ;[1 0.848 0.3919] Client: Equip Armor
  (Class|SkinnedMeshComponent|SetSkeletalMesh _returnvalue _equippedmesh true)
  (Rendering|Material|SetMaterial _returnvalue 0 (select (Utilities|IsValid _materialoverride) _materialoverride (.MaterialInterface (Utilities|Struct|BreakSkeletalMaterial (Utilities|Array|Get(acopy) (Variables|/Script/Engine.SkeletalMesh|GetMaterials _equippedmesh)))))))

(event EventAttackFx
  ;[0.6761 0.4477 1] Attack Fx
  (Animation|PlayAnimMontage "/Game/MMO/Characters/Mannequin/Animations/AM_Punch.AM_Punch" 1.0 "None"))

(event EventOnBecomeViewTarget
  (params (PC :type Player%20Controller%20Object%20Reference))
  ;[1 1 1] OnBecomeViewTarget -  Allow clicking through own character
  (|CallParentFunction PC)
  (Networking|CanExecuteCosmeticEvents
    (:True
      (Collision|SetCollisionResponsetoChannel (Variables|Default|GetCapsuleComponent) "ECC_Visibility" "ECR_Ignore"))))

(event EventBeginPlay
  ;[1 1 1] Begin play
  (|CallParentFunction)
  (Networking|CanExecuteCosmeticEvents
    (:True
      ;[1 1 1] make body parts use the pose of the main mesh
      (Class|SkinnedMeshComponent|SetMasterPoseComponent (Variables|Default|GetFeet) (Variables|Character|GetMesh) false)
      ;[0.7856 0.6477 1] Create material instances for body parts (for highlight)
      (for _array_element (Utilities|Array|MakeArray (Variables|Default|GetHead) (Variables|Default|GetLegs) (Variables|Default|GetHands) (Variables|Default|GetFeet))
        (bind _returnvalue (Rendering|Material|CreateDynamicMaterialInstance _array_element 0 0 "None" :!class /Script/Engine.PrimitiveComponent))
        (Utilities|Array|Add (Variables|Default|GetDynamicMaterialInstances) _returnvalue)))))

(event EventEquipItem
  (params (Equipment :type Equipment%20Object%20Reference))
  ;[1 0.848 0.3919] EquipItem
  (Utilities|FlowControl|Sequence
    (:then_0
      (switch Utilities|FlowControl|Switch|SwitchonEquipmentType (Variables|/Script/MMO.Equipment|GetType Equipment)
        (:Head
          (Variables|Default|SetEquippedHead Equipment))
        (:Torso
          (Variables|Default|SetEquippedChest Equipment))
        (:Legs
          (Variables|Default|SetEquippedLegs Equipment))
        (:Hands
          (Variables|Default|SetEquippedHands Equipment))
        (:Feet
          (Variables|Default|SetEquippedFeet Equipment))))
    (:then_1
      (CallFunction|ConfirmEquip (Utilities|Struct|MakeFInventoryItem Equipment 1)))))

(event Input|KeyboardEvents|1
  (params (Key :type Key%20Structure))
  ;[0.3281 0.8359 1] Hotbar keys
  (:Pressed
    (CallFunction|UseHotbarSlot 0 (Variables|Default|GetCurrentTarget))))

(event Input|KeyboardEvents|2
  (params (Key :type Key%20Structure))
  ;[0.3281 0.8359 1] Hotbar keys
  (:Pressed
    (CallFunction|UseHotbarSlot 1 (Variables|Default|GetCurrentTarget))))

(event Input|KeyboardEvents|3
  (params (Key :type Key%20Structure))
  ;[0.3281 0.8359 1] Hotbar keys
  (:Pressed
    (CallFunction|UseHotbarSlot 2 (Variables|Default|GetCurrentTarget))))

(event Input|KeyboardEvents|4
  (params (Key :type Key%20Structure))
  ;[0.3281 0.8359 1] Hotbar keys
  (:Pressed
    (CallFunction|UseHotbarSlot 3 (Variables|Default|GetCurrentTarget))))

(fn ConstructionScript
  (|CallParentFunction)
  (Class|SkinnedMeshComponent|SetMasterPoseComponent (Variables|Default|GetLegs) (Variables|Character|GetMesh) false))

(fn OnRepEquippedHead
  (bind _equippedhead (Variables|Default|GetEquippedHead))
  (Utilities|IsValid _equippedhead
    (:Is%20Valid
      (CallFunction|EquipArmor _equippedhead))
    (:Is%20Not%20Valid
      (CallFunction|EquipUnderwear "Head"))))

(fn OnRepEquippedHands
  (bind _equippedhands (Variables|Default|GetEquippedHands))
  (Utilities|IsValid _equippedhands
    (:Is%20Valid
      (CallFunction|EquipArmor _equippedhands))
    (:Is%20Not%20Valid
      (CallFunction|EquipUnderwear "Hands"))))

(fn OnRepEquippedFeet
  (bind _equippedfeet (Variables|Default|GetEquippedFeet))
  (Utilities|IsValid _equippedfeet
    (:Is%20Valid
      (CallFunction|EquipArmor _equippedfeet))
    (:Is%20Not%20Valid
      (CallFunction|EquipUnderwear "Feet"))))

(fn OnRepEquippedLegs
  (bind _equippedlegs (Variables|Default|GetEquippedLegs))
  (Utilities|IsValid _equippedlegs
    (:Is%20Valid
      (CallFunction|EquipArmor _equippedlegs))
    (:Is%20Not%20Valid
      (CallFunction|EquipUnderwear "Legs"))))

(fn OnRepEquippedChest
  (bind _equippedchest (Variables|Default|GetEquippedChest))
  (Utilities|IsValid _equippedchest
    (:Is%20Valid
      (CallFunction|EquipArmor _equippedchest))
    (:Is%20Not%20Valid
      (CallFunction|EquipUnderwear "Torso"))))

(fn UseHotbarItem
  (params (Item :type Item%20Data%20Object%20Reference))
  ;[1 0.6005 0.1372] Find this item in the inventory and use it
  (bind _array_element (Utilities|Array|ForEachLoopwithBreak (Variables|Default|GetInventory) :!label _label)
    (:LoopBody
      (if (== (.Item (Utilities|Struct|BreakFInventoryItem _array_element)) Item)
        (CallFunction|UseItem (.SlotNumber (Utilities|Struct|BreakFInventoryItem _array_element)))
        (goto _label Break)))))

(fn GetEquippedItem
  (params (EquipmentType :type EquipmentType%20Enum :default "Head"))
  (return (Utilities|Select :Index EquipmentType :Head (Variables|Default|GetEquippedHead) :Torso (Variables|Default|GetEquippedChest) :Legs (Variables|Default|GetEquippedLegs) :Hands (Variables|Default|GetEquippedHands) :Feet (Variables|Default|GetEquippedFeet) :Weapon 0 :WeaponSecondary 0)))